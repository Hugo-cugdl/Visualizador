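; BP_ColorChange_Object is an object of five cube meshes whose material switches between two color material instances.
; The construction script picks the starting material from ColorToggle, and two custom events swap slot 0 on all five cubes.
; BeginPlay creates dynamic materials for the first Cube only, then SetValues applies Color, Roughness and Metallic to them.
; The swap events assign the plain instances without reapplying those parameters.
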(event Custom|SetValues
  (for _array_element (Variables|Default|GetDynamic%20Materials)
    (Rendering|Material|SetVectorParameterValue _array_element "Color" (Variables|Default|GetColor) :!class /Script/Engine.MaterialInstanceDynamic)
    (Rendering|Material|SetScalarParameterValue _array_element "Roughness" (Variables|Default|GetRoughness) :!class /Script/Engine.MaterialInstanceDynamic)
    (Rendering|Material|SetScalarParameterValue _array_element "Metallic" (Variables|Default|GetMetallic) :!class /Script/Engine.MaterialInstanceDynamic)))

(event Custom|Mat1Change_Event
  (Rendering|Material|SetMaterial (Variables|Default|GetCube) 0 "/Game/MI_ColorMaterial_1.MI_ColorMaterial_1"))

(event Custom|Mat2Change_Event
  (Rendering|Material|SetMaterial (Variables|Default|GetCube) 0 "/Game/MI_ColorMaterial_2.MI_ColorMaterial_2"))

(event EventBeginPlay
  (bind _cube (Variables|Default|GetCube))
  (for (_array_element _array_index) (Rendering|Material|GetMaterials _cube)
    (bind _returnvalue (Rendering|Material|CreateDynamicMaterialInstance _cube _array_index _array_element "None" :!class /Script/Engine.PrimitiveComponent))
    (Utilities|Array|SetArrayElem (Variables|Default|GetDynamic%20Materials) _array_index _returnvalue true))
  (CallFunction|SetValues))

(fn ConstructionScript
  (if (Variables|Default|GetColorToggle)
    (Rendering|Material|SetMaterial (Variables|Default|GetCube) 0 "/Game/MI_ColorMaterial_1.MI_ColorMaterial_1")
    (else
      (Rendering|Material|SetMaterial (Variables|Default|GetCube) 0 "/Game/MI_ColorMaterial_2.MI_ColorMaterial_2"))))
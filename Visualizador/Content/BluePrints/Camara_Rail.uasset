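; Camera rail Blueprint that moves a camera along a spline path.
; The construction script places the camera at the PosONRail fraction of the spline's length, so its position follows that value at construction.
; Start_Anim_Event plays a timeline from the start, using its Orbital track as the fraction of spline length to update the camera's world location.
; Only location is driven; rotation is left untouched.
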(event Custom|Start_Anim_Event
  (bind _orbital (Timeline|Timeline PlayFromStart)
    (:Update
      (Transformation|SetWorldLocation (Variables|/Script/Engine.Actor|GetRootComponent (Variables|Default|GetCamera)) (Spline|GetLocationatDistanceAlongSpline (Variables|Default|GetSpline) (* _orbital (Spline|GetSplineLength (Variables|Default|GetSpline))) "World") false false))))

(fn ConstructionScript
  (Transformation|SetWorldLocation (Variables|/Script/Engine.Actor|GetRootComponent (Variables|Default|GetCamera)) (Spline|GetLocationatDistanceAlongSpline (Variables|Default|GetSpline) (* (Variables|Default|GetPos_ON_rail) (Spline|GetSplineLength (Variables|Default|GetSpline))) "World") false false))